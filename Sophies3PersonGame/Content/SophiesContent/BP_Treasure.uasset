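; BP_Treasure is a pickup actor that awards points to the player when interacted with.
; On BeginPlay it caches a BP_ThirdPersonCharacter reference, keeping the last one found, and its SphereCollision overlaps toggle whether that character can interact.
; Every Tick it polls the character's IsInteracting flag while in range, then adds its Points to the character's total, prints that total and destroys itself.
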(event OnComponentBeginOverlap(SphereCollision)
  (params (OverlappedComponent :type Primitive%20Component%20Object%20Reference) (OtherActor :type Actor%20Object%20Reference) (OtherComp :type Primitive%20Component%20Object%20Reference) (OtherBodyIndex :type Integer) (bFromSweep :type Boolean) (SweepResult :type Hit%20Result%20Structure%20%28by%20ref%29))
  (CallFunction|CheckifPlayer OtherActor true))

(event OnComponentEndOverlap(SphereCollision)
  (params (OverlappedComponent :type Primitive%20Component%20Object%20Reference) (OtherActor :type Actor%20Object%20Reference) (OtherComp :type Primitive%20Component%20Object%20Reference) (OtherBodyIndex :type Integer))
  (CallFunction|CheckifPlayer OtherActor false))

(event EventBeginPlay
  (bind _outactors (Actor|GetAllActorsOfClass "/Game/ThirdPerson/Blueprints/BP_ThirdPersonCharacter.BP_ThirdPersonCharacter_C"))
  (for _array_element _outactors
    (Variables|Default|SetPlayer _array_element)))

(event Collision|EventActorBeginOverlap
  (params (OtherActor :type Actor%20Object%20Reference)))

(event EventTick
  (params (DeltaSeconds :type Float%20%28single-precision%29))
  (CallFunction|GivePoints))

(fn ConstructionScript)

(fn GivePoints
  (if (and (Variables|Default|GetCanBeInteracted) (Variables|/Game/ThirdPerson/Blueprints/BP_ThirdPersonCharacter.BP_ThirdPersonCharacter_C|GetIsInteracting (Variables|Default|GetPlayer)))
    (bind _output_get (Variables|/Game/ThirdPerson/Blueprints/BP_ThirdPersonCharacter.BP_ThirdPersonCharacter_C|SetPoints (Variables|Default|GetPlayer) (+ (Variables|/Game/ThirdPerson/Blueprints/BP_ThirdPersonCharacter.BP_ThirdPersonCharacter_C|GetPoints (Variables|Default|GetPlayer)) (Variables|Default|GetPoints))))
    (Development|PrintString (Utilities|String|ToString(Integer) _output_get))
    (Actor|DestroyActor)))

(fn CheckifPlayer
  (params (Actor :type Actor%20Object%20Reference) (Interact :type Boolean))
  (if (== Actor (Variables|Default|GetPlayer))
    (Variables|Default|SetCanBeInteracted Interact)))